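; Camera rail actor for authoring a list of camera points along the CamLocSpline spline, each with a target location, spline time and weight.
; Events add points sorted by spline time, remove, save and step through them, loading the selected point into editable variables.
; Construction rebuilds camera ports for the spline ends and a preview camera at OverviewTravel aimed at TargetLocation.
; The getter functions return only placeholder values.
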(event Custom|AddCamPoint
  (bind _newindex (CallFunction|AddCameraPoint (Variables|PasTouche|GetCameraPoints) (Spline|GetLocationatTime (Variables|Default|GetCamLocSpline) (Variables|Touche|GetOverviewTravel) "Local" false) (Variables|Touche|GetOverviewTravel) (Variables|Touche|GetWeight) 0.0))
  (Variables|PasTouche|SetCurrentPointIndex _newindex))

(event Custom|RemoveCamPoint
  (Utilities|Array|RemoveIndex (Variables|PasTouche|GetCameraPoints) (Variables|PasTouche|GetCurrentPointIndex))
  (bind _changed (CallFunction|ChangeIndex))
  (if _changed
    (CallFunction|RefreshVariables :!label _label)
    (else
      (bind _changed_2 (CallFunction|ChangeIndex -1))
      (if _changed_2
        (goto _label)
        (else
          (CallFunction|ChangeIndex 1)
          (CallFunction|RefreshVariables))))))

(event Custom|NextPoint
  (bind (_changed _value) (CallFunction|ChangeIndex 1))
  (if _changed
    (Variables|PasTouche|SetCurrentPointIndex _value)
    (CallFunction|RefreshVariables)))

(event Custom|PrevoiusPoint
  (bind (_changed _value) (CallFunction|ChangeIndex -1))
  (if _changed
    (Variables|PasTouche|SetCurrentPointIndex _value)
    (CallFunction|RefreshVariables)))

(event Custom|_RefreshVariables
  (bind _currentpointindex (Variables|PasTouche|GetCurrentPointIndex))
  (bind _camerapoints (Variables|PasTouche|GetCameraPoints))
  (bind _output (Utilities|Array|Get(acopy) _camerapoints _currentpointindex))
  (Variables|Touche|SetWeight (.weight _output))
  (Variables|Touche|SetTargetPlayer false)
  (Variables|PasTouche|SetTargetLocation (.targetlocation _output))
  (Variables|Touche|SetOverviewTravel (.splinetime _output))
  (CallFunction|Construct))

(event Custom|Save
  (Utilities|Array|SetArrayElem (Variables|PasTouche|GetCameraPoints) (Variables|PasTouche|GetCurrentPointIndex) (Utilities|Struct|MakeSTR_CameraPoint (Variables|PasTouche|GetTargetLocation) (Variables|Touche|GetOverviewTravel) (Variables|Touche|GetWeight) 0.0)))

(event Custom|Construct
  (bind _camlocspline (Variables|Default|GetCamLocSpline))
  (bind _cameraports (Variables|PasTouche|GetCameraPorts))
  (bind _camlocspline_2 (Variables|Default|GetCamLocSpline))
  (bind _overviewtravel (Variables|Touche|GetOverviewTravel))
  (bind _returnvalue (Spline|GetLocationatTime _camlocspline_2 _overviewtravel "Local" false))
  (Utilities|Array|Clear (Variables|PasTouche|GetCameraPorts))
  (for _array_element (Actor|GetComponentsByClass "/Script/Engine.CameraComponent")
    (Components|DestroyComponent _array_element))
  (Utilities|FlowControl|Sequence
    (:then_0
      (bind _returnvalue_2 (AddComponent|AddSCCameraPort false (Math|Conversions|ToTransform(Vector) (Spline|GetLocationatSplinePoint _camlocspline 0 "Local"))))
      (bind _returnvalue_3 (AddComponent|AddSCCameraPort false (Math|Conversions|ToTransform(Vector) (Spline|GetLocationatSplinePoint _camlocspline (Spline|GetNumberOfSplinePoints _camlocspline) "Local"))))
      (Utilities|Array|Add _cameraports _returnvalue_3)
      (Utilities|Array|Add _cameraports _returnvalue_2))
    (:then_2
      (AddComponent|AddCameraComponent false (Math|Transform|MakeTransform _returnvalue (Math|Conversions|RotationFromXVector (- (Variables|PasTouche|GetTargetLocation) _returnvalue)) "1.000000,1.000000,1.000000"))
      (AddComponent|AddStaticMeshComponent false (Math|Transform|MakeTransform "0, 0, 0" "0, 0, 0" "0.100000,0.100000,0.100000")))))

(fn ConstructionScript
  (CallFunction|Construct)
  (for _array_element (Variables|PasTouche|GetCameraPorts)
    (AddComponent|AddStaticMeshComponent false (Math|Transform|MakeTransform (Variables|/Script/Engine.SceneComponent|GetRelativeLocation _array_element) "0, 0, 0" "0.500000,0.500000,0.500000"))))

(fn AddCameraPoint
  (params (TargetArray :type Array%20of%20STR%20Camera%20Point%20Structures) (Target%20Location :type Vector) (Spline%20Time :type Float%20%28double-precision%29) (Weight :type Float%20%28double-precision%29) (TrackPlayerBlend :type Float%20%28double-precision%29))
  (bind _str_camerapoint (Utilities|Struct|MakeSTR_CameraPoint Target%20Location Spline%20Time Weight TrackPlayerBlend))
  (for (_array_element _array_index) TargetArray
    (if (< Spline%20Time (.SplineTime (Utilities|Struct|BreakSTR_CameraPoint _array_element)))
      (Utilities|Array|Insert TargetArray _str_camerapoint _array_index)
      (return _array_index)))
  (bind _returnvalue (Utilities|Array|Add TargetArray _str_camerapoint))
  (return _returnvalue))

(fn ChangeIndex
  (params (Delta :type Integer))
  (bind _currentpointindex (Variables|PasTouche|GetCurrentPointIndex))
  (bind _camerapoints (Variables|PasTouche|GetCameraPoints))
  (bind _returnvalue (Utilities|Array|LastIndex _camerapoints))
  (bind _returnvalue_2 (+ _currentpointindex Delta))
  (bind _returnvalue_3 (< _returnvalue_2 0))
  (bind _returnvalue_4 (> _returnvalue_2 _returnvalue))
  (bind _returnvalue_5 (or _returnvalue_3 _returnvalue_4))
  (bind _returnvalue_6 (not _returnvalue_5))
  (return _returnvalue_6 (Math|Integer|SelectInt _returnvalue_2 _currentpointindex _returnvalue_6)))

(fn CheckonPoint
  (return false))

(fn GetOverview
  (return 0.0))

(fn GetToolType
  (return "NewEnumerator0"))

(fn GetTrackBlend
  (return 0.0))

(fn GetWeight
  (return 0.0))