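; Cine camera manager component that drives a rail-following camera position from the third-person player's progress along a player rail.
; Each tick it maps the player's closest spline point to a time, smooths it, samples the paired camera rail and writes the result to the character's Loc variable.
; When the player strays past a rail end, a DoOnce with delayed reset re-picks both rails via the nearest BP_Switcher's parent.
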(event EventBeginPlay
  (bind _asbp_third_person_character (Utilities|Casting|CastToBP_ThirdPersonCharacter (Game|GetPlayerCharacter 0)))
  (Variables|Default|SetPlayerRef _asbp_third_person_character)
  (Variables|Default|GetFollowedCameraRail
    (:then)
    (:else
      (bind _outactors (Actor|GetAllActorsOfClass "/Game/NewCineTool/BP_Switcher.BP_Switcher_C"))
      (Variables|Default|SetFollowedPlayerRail (.AsBP%20Cine%20Player%20Rail (Utilities|Casting|CastToBP_CinePlayerRail (Actor|GetParentActor (.ReturnValue (Actor|FindNearestActor (Transformation|GetActorLocation (Variables|Default|GetPlayerRef)) _outactors))))))
      (Variables|Default|SetFollowedCameraRail (Variables|/Game/NewCineTool/BP_CinePlayerRail.BP_CinePlayerRail_C|GetCineCamRail (.AsBP%20Cine%20Player%20Rail (Utilities|Casting|CastToBP_CinePlayerRail (Actor|GetParentActor (.ReturnValue (Actor|FindNearestActor (Transformation|GetActorLocation (Variables|Default|GetPlayerRef)) _outactors))))))))))

(event EventTick
  (params (DeltaSeconds :type Float%20%28single-precision%29))
  (bind _followedplayerrail (Variables|Default|GetFollowedPlayerRail))
  (bind _followedplayerrail_2 (Variables|Default|GetFollowedPlayerRail))
  (bind _spline (Variables|/Game/NewCineTool/BP_CinePlayerRail.BP_CinePlayerRail_C|GetSpline _followedplayerrail))
  (Variables|Default|SetDelta%20Seconds DeltaSeconds)
  (bind _output_get (Variables|Default|SetTargetTimeOnCameraRail (Class|SplineComponent|GetTimeatDistanceAlongSpline _spline (Class|SplineComponent|GetDistanceAlongSplineatLocation _spline (Spline|FindLocationClosesttoWorldLocation _spline (Transformation|GetActorLocation (Variables|Default|GetPlayerRef)) "Local") "Local"))))
  (bind _output_get_2 (Variables|Default|SetSmoothedTimeOnCameraRail (Math|Interpolation|FInterpTo (Variables|Default|GetSmoothedTimeOnCameraRail) _output_get (Variables|Default|GetDelta%20Seconds) 2.0)))
  (bind _output_get_3 (Variables|Default|SetSmoothedCameraLocation (Spline|GetLocationatTime (Variables|/Game/NewCineTool/BP_CineCam_Rail.BP_CineCam_Rail_C|GetSpline (Variables|Default|GetFollowedCameraRail)) _output_get_2 "World" false)))
  (Variables|/Game/ThirdPerson/Blueprints/BP_ThirdPersonCharacter.BP_ThirdPersonCharacter_C|SetLoc (Variables|Default|GetPlayerRef) _output_get_3)
  (if (or (== (Variables|Default|GetTargetTimeOnCameraRail) 1.0) (== (Variables|Default|GetTargetTimeOnCameraRail) 0.0))
    (if (> (Math|Vector|Distance(Vector) (Transformation|GetWorldLocation (select (== (Variables|Default|GetTargetTimeOnCameraRail) 1.0) (Variables|/Game/NewCineTool/BP_CinePlayerRail.BP_CinePlayerRail_C|Getend _followedplayerrail_2) (Variables|/Game/NewCineTool/BP_CinePlayerRail.BP_CinePlayerRail_C|Getstart _followedplayerrail_2))) (Transformation|GetActorLocation (Variables|Default|GetPlayerRef))) 1e+02)
      (Utilities|FlowControl|DoOnce false :!label _label
        (:Completed
          (Utilities|FlowControl|Sequence
            (:then_0
              (Utilities|FlowControl|Delay 1.0)
              (goto _label Reset))
            (:then_1
              (CallFunction|SwitchtoNearestSpline))))))))

(fn SwitchtoNearestSpline
  (bind _outactors (Actor|GetAllActorsOfClass "/Game/NewCineTool/BP_Switcher.BP_Switcher_C"))
  (Utilities|Set|RemoveItems (Utilities|Set|MakeSet (.AsBP%20Switcher (Utilities|Casting|CastToBP_Switcher (Variables|/Script/Engine.ChildActorComponent|GetChildActor (Variables|/Game/NewCineTool/BP_CinePlayerRail.BP_CinePlayerRail_C|GetBP_Switcher (Variables|Default|GetFollowedPlayerRail))))) (.AsBP%20Switcher (Utilities|Casting|CastToBP_Switcher (Variables|/Script/Engine.ChildActorComponent|GetChildActor (Variables|/Game/NewCineTool/BP_CinePlayerRail.BP_CinePlayerRail_C|GetBP_Switcher1 (Variables|Default|GetFollowedPlayerRail)))))) _outactors)
  (Variables|Default|SetFollowedPlayerRail (.AsBP%20Cine%20Player%20Rail (Utilities|Casting|CastToBP_CinePlayerRail (Actor|GetParentActor (.ReturnValue (Actor|FindNearestActor (Transformation|GetActorLocation (Variables|Default|GetPlayerRef)) _outactors))))))
  (Variables|Default|SetFollowedCameraRail (Variables|/Game/NewCineTool/BP_CinePlayerRail.BP_CinePlayerRail_C|GetCineCamRail (.AsBP%20Cine%20Player%20Rail (Utilities|Casting|CastToBP_CinePlayerRail (Actor|GetParentActor (.ReturnValue (Actor|FindNearestActor (Transformation|GetActorLocation (Variables|Default|GetPlayerRef)) _outactors))))))))