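; Camera point actor for a cinematic rail tool, pairing a position on a rail's spline with an aim direction toward the actor.
; Rebuild moves SplineLoc to PositionOnRail on the rail spline and rotates Camera along the vector from there to the actor's location.
; The construction script calls Rebuild and keeps the point registered in its rail's CineCamPoints, using PreviousRail to unregister when the reference changes or clears.
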(event Custom|Rebuild
  (Transformation|SetWorldLocation (Variables|Default|GetsplineLoc) (Spline|GetLocationatTime (Variables|/Game/NewCineTool/BP_CineCam_Rail.BP_CineCam_Rail_C|GetSpline (Variables|Default|GetCineRail_Ref)) (Variables|Default|GetPosition%20On%20Rail) "World" false) false false)
  (Transformation|SetWorldRotation (Variables|Default|GetCamera) (Math|Conversions|RotationFromXVector (- (Transformation|GetActorLocation) (Transformation|GetWorldLocation (Variables|Default|GetsplineLoc)))) false false))

(event EventBeginPlay)

(event Collision|EventActorBeginOverlap
  (params (OtherActor :type Actor%20Object%20Reference)))

(event EventTick
  (params (DeltaSeconds :type Float%20%28single-precision%29)))

(fn ConstructionScript
  (bind _cinerail_ref (Variables|Default|GetCineRail_Ref))
  (bind _cinecampoints (Variables|/Game/NewCineTool/BP_CineCam_Rail.BP_CineCam_Rail_C|GetCineCamPoints _cinerail_ref))
  (bind _cinerail_ref_2 (Variables|Default|GetCineRail_Ref)
    (:then
      (bind _previous_rail (Variables|Default|Getprevious_rail)
        (:then
          (if (== _cinerail_ref_2 _previous_rail)
            (CallFunction|Rebuild)
            (else
              (Utilities|Array|RemoveItem (Variables|/Game/NewCineTool/BP_CineCam_Rail.BP_CineCam_Rail_C|GetCineCamPoints (Variables|Default|Getprevious_rail)) self :!label _label)
              (Variables|Default|Setprevious_rail _cinerail_ref)
              (for _array_element _cinecampoints
                (if (== _array_element self)
                  (Utilities|Array|RemoveItem (Variables|/Game/NewCineTool/BP_CineCam_Rail.BP_CineCam_Rail_C|GetCineCamPoints (Variables|Default|GetCineRail_Ref)) self)))
              (Utilities|Array|AddUnique _cinecampoints self)
              (CallFunction|Rebuild))))
        (:else
          (goto _label))))
    (:else
      (bind _previous_rail_2 (Variables|Default|Getprevious_rail)
        (:then
          (Utilities|Array|RemoveItem (Variables|/Game/NewCineTool/BP_CineCam_Rail.BP_CineCam_Rail_C|GetCineCamPoints _previous_rail_2) self)
          (Variables|Default|Setprevious_rail 0))
        (:else)))))