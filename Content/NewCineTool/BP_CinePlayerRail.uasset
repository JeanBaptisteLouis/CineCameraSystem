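; BP_CinePlayerRail is a spline-based rail actor in the cine tool, apparently for guiding the player.
; The construction script snaps the Start and End components to the spline's local positions at time 0 and 1.
; It also flags the StartSwitcher child BP_Switcher as the start switcher.
; The event graph holds no active logic, so this Blueprint only handles setup.
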(event EventBeginPlay)

(event Collision|EventActorBeginOverlap
  (params (OtherActor :type Actor%20Object%20Reference)))

(event EventTick
  (params (DeltaSeconds :type Float%20%28single-precision%29)))

(fn ConstructionScript
  (bind _spline (Variables|Default|GetSpline))
  (Transformation|SetRelativeLocation (Variables|Default|Getstart) (Spline|GetLocationatTime _spline 0.0 "Local" false) false false)
  (Variables|/Game/NewCineTool/BP_Switcher.BP_Switcher_C|SetisStart (.AsBP%20Switcher (Utilities|Casting|CastToBP_Switcher (Variables|/Script/Engine.ChildActorComponent|GetChildActor (Variables|Default|Getstart_Switcher)))) true)
  (Transformation|SetRelativeLocation (Variables|Default|Getend) (Spline|GetLocationatTime _spline 1.0 "Local" false) false false))